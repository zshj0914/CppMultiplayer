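; Multiplayer game mode Blueprint that exercises a socket connection owned by BP_PuzzlePlatformsGameInstance.
; On BeginPlay it creates a socket to a hardcoded IP and port, starts a looping timer and calls SocketReceive once.
; Each timer tick, if socket creation succeeded, sends a numbered "UE4 num:" text message through the game instance and increments the counter.
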(event Custom|SendMessage
  (bind _index (Variables|Default|GetIndex))
  (if (Variables|Default|GetSuccess)
    (bind _asbp_puzzle_platforms_game_instance (Utilities|Casting|CastToBP_PuzzlePlatformsGameInstance (Game|GetGameInstance)))
    (Class|PuzzlePlatformsGameInstance|SocketSend _asbp_puzzle_platforms_game_instance (Utilities|String|Append "UE4 num:" (Utilities|String|ToString(Integer) _index)))
    (Math|Integer|IncrementInt _index)))

(event EventBeginPlay
  (bind _asbp_puzzle_platforms_game_instance (Utilities|Casting|CastToBP_PuzzlePlatformsGameInstance (Game|GetGameInstance)))
  (bind _returnvalue (Class|PuzzlePlatformsGameInstance|SocketCreate _asbp_puzzle_platforms_game_instance "127.0.0.0" 4399))
  (Variables|Default|SetSuccess _returnvalue)
  (Utilities|Time|SetTimerbyEvent (delegate Custom|SendMessage) 2.0 true)
  (Class|PuzzlePlatformsGameInstance|SocketReceive _asbp_puzzle_platforms_game_instance))

(event EventTick
  (params (DeltaSeconds :type Float%20%28single-precision%29)))

(fn ConstructionScript)